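; Test Blueprint that checks whether the RapidLib machine learning plugin DLL loads and works, reporting each stage through printed strings.
; BeginPlay imports the DLL from the RapidLib folder, creates a regression model and prints its JSON, with failure messages for either step.
; EndPlay calls DestroyModel with a literal zero rather than the created handle, as the node storing it in Test is never executed.
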(event `self.ReceiveBeginPlay`
  (`KismetSystemLibrary.PrintString` "Hello")
  (bind _returnvalue (`InteractML.importDLL` "RapidLib" "RapidLibPlugin.dll"))
  (if _returnvalue
    (`KismetSystemLibrary.PrintString` "dll loaded")
    (bind _returnvalue_2 (`InteractML.createRegressionModel`))
    (if (!= _returnvalue_2 0)
      (`KismetSystemLibrary.PrintString` "created a regression model")
      (bind _returnvalue_3 (`InteractML.getJSON` _returnvalue_2))
      (`KismetSystemLibrary.PrintString` _returnvalue_3)
      (else
        (`KismetSystemLibrary.PrintString` "failed to create a regression model")))
    (else
      (`KismetSystemLibrary.PrintString` "failed to load dll"))))

(event `self.ReceiveEndPlay`
  (params (EndPlayReason :type "EEndPlayReason Enum" :default "Destroyed"))
  (`InteractML.destroyModel` 0))

(fn `UserConstructionScript`)